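; Tank AI controller Blueprint with a helper for locating health pickups.
; FindClosestHealth loops over every MyHPPickupBP actor and returns the nearest one to itself that is farther than MinDistance and closer than the starting ClosestDistance.
; BeginPlay only prints a startup message, and nothing in this Blueprint calls the search.
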(event `self.ReceiveBeginPlay`
  (`KismetSystemLibrary.PrintString` "starting"))

(fn `FindClosestHealth`
  (returns (ClosestPack :type "Actor Object Reference"))
  (bind _outactors (`GameplayStatics.GetAllActorsOfClass` "/Game/Pickups/MyHPPickupBP.MyHPPickupBP_C"))
  (for _array_element _outactors
    (bind _returnvalue (`self.GetDistanceTo` _array_element))
    (if (and (< _returnvalue (`self.ClosestDistance`)) (> _returnvalue (`self.MinDistance`)))
      (set `self.ClosestPack` _array_element)
      (set `self.ClosestDistance` _returnvalue)))
  (return (`self.ClosestPack`)))

(fn `UserConstructionScript`)